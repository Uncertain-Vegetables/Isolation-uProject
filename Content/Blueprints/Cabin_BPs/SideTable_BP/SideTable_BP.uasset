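; Interactive side table Blueprint for the cabin, with a drawer the player can slide open and closed.
; A trigger box enables input on overlap and disables it on exit, so the Action input only works while something is inside the box.
; Each press toggles a closed flag and uses MoveComponentTo to slide the drawer to a fixed open offset or back to its starting location, cached in the construction script.
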(event `self.Box.OnComponentBeginOverlap`
  (params (OverlappedComponent :type "PrimitiveComponent Object Reference") (OtherActor :type "Actor Object Reference") (OtherComp :type "PrimitiveComponent Object Reference") (OtherBodyIndex :type Integer) (bFromSweep :type Boolean) (SweepResult :type "HitResult Structure (by ref)"))
  (`self.EnableInput` (`GameplayStatics.GetPlayerController` 0)))

(event `InputAction|Action`
  (params (Key :type "Key Structure"))
  (bind _smallsidetable_drawer (`self.SmallSideTable_Drawer`))
  (:`Pressed`
    (if (`self.DrawerClosed`)
      (`KismetSystemLibrary.MoveComponentTo` _smallsidetable_drawer (0.0 -35.0 0.0) (struct) false false 0.5)
      (set `self.DrawerClosed` false)
      (else
        (`KismetSystemLibrary.MoveComponentTo` _smallsidetable_drawer (`self.RelativePos`) (struct) false false 0.5)
        (set `self.DrawerClosed` true)))))

(event `self.Box.OnComponentEndOverlap`
  (params (OverlappedComponent :type "PrimitiveComponent Object Reference") (OtherActor :type "Actor Object Reference") (OtherComp :type "PrimitiveComponent Object Reference") (OtherBodyIndex :type Integer))
  (`self.DisableInput` (`GameplayStatics.GetPlayerController` 0)))

(fn `UserConstructionScript`
  (set `self.RelativePos` (`SceneComponent.RelativeLocation` (`self.SmallSideTable_Drawer`))))