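; Interactable cabin stove whose door the player swings open and shut with the Action input.
; A Box trigger enables player 0's input on any overlap and disables it when the overlap ends.
; Each press plays the Furnace sound and toggles DoorOpen, using MoveComponentTo to rotate StoveDoor between a fixed open angle and the rotation cached in the construction script.
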(event `self.Box.OnComponentBeginOverlap`
  (params (OverlappedComponent :type "PrimitiveComponent Object Reference") (OtherActor :type "Actor Object Reference") (OtherComp :type "PrimitiveComponent Object Reference") (OtherBodyIndex :type Integer) (bFromSweep :type Boolean) (SweepResult :type "HitResult Structure (by ref)"))
  (`self.EnableInput` (`GameplayStatics.GetPlayerController` 0)))

(event `self.Box.OnComponentEndOverlap`
  (params (OverlappedComponent :type "PrimitiveComponent Object Reference") (OtherActor :type "Actor Object Reference") (OtherComp :type "PrimitiveComponent Object Reference") (OtherBodyIndex :type Integer))
  (`self.DisableInput` (`GameplayStatics.GetPlayerController` 0)))

(event `InputAction|Action`
  (params (Key :type "Key Structure"))
  (bind _stove_door (`self.stove_door`))
  (:`Pressed`
    (if (`self.DoorOpen`)
      (`GameplayStatics.PlaySound2D` "/Game/Sounds/Furnace/Furnace.Furnace" 1.0 1.0 0.0 null null)
      (`KismetSystemLibrary.MoveComponentTo` _stove_door (0.0 0.0 0.0) (`self.RelativeRot`) false false 1.0)
      (set `self.DoorOpen` false)
      (else
        (`GameplayStatics.PlaySound2D` "/Game/Sounds/Furnace/Furnace.Furnace" 1.0 1.0 0.0 null null)
        (`KismetSystemLibrary.MoveComponentTo` _stove_door (0.0 0.0 0.0) (struct :`Yaw` -90.0) false false 1.0)
        (set `self.DoorOpen` true)))))

(fn `UserConstructionScript`
  (set `self.RelativeRot` (`SceneComponent.RelativeRotation` (`self.stove_door`))))