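; Exit door Blueprint that swings its Door component and loads the "Landscape" level when the player uses it.
; Box overlap enables player input on the door, and leaving the box disables it.
; The Action press, gated on DoorClosed being false, rotates the door with MoveComponentTo, then opens the level after a short delay.
; BeginPlay also runs a timed door move, and the construction script caches the door's relative location.
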(event `self.ReceiveBeginPlay`
  (`KismetSystemLibrary.MoveComponentTo` (`self.Door`) (0.0 0.0 0.0) (struct) false false 1.5))

(event `self.Box.OnComponentBeginOverlap`
  (params (OverlappedComponent :type "PrimitiveComponent Object Reference") (OtherActor :type "Actor Object Reference") (OtherComp :type "PrimitiveComponent Object Reference") (OtherBodyIndex :type Integer) (bFromSweep :type Boolean) (SweepResult :type "HitResult Structure (by ref)"))
  (`self.EnableInput` (`GameplayStatics.GetPlayerController` 0)))

(event `InputAction|Action`
  (params (Key :type "Key Structure"))
  (:`Pressed`
    (if (not (`self.DoorClosed`))
      (`KismetSystemLibrary.MoveComponentTo` (`self.Door`) (0.0 0.0 0.0) (struct :`Yaw` 10.0) false false 1.0)
      (set `self.Doorclosed` false)
      (`KismetSystemLibrary.Delay` 1.7)
      (`GameplayStatics.OpenLevel` "Landscape"))))

(event `self.Box.OnComponentEndOverlap`
  (params (OverlappedComponent :type "PrimitiveComponent Object Reference") (OtherActor :type "Actor Object Reference") (OtherComp :type "PrimitiveComponent Object Reference") (OtherBodyIndex :type Integer))
  (`self.DisableInput` (`GameplayStatics.GetPlayerController` 0)))

(fn `UserConstructionScript`
  (set `self.Door_Rel_Pos` (`SceneComponent.RelativeLocation` (`self.Door`))))