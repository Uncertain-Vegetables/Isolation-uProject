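; Snow trail capture actor that follows the player and maintains render targets for snow trails.
; Tick pushes the capture width to SnowMpc, creates the persistence material instance and clears both render targets.
; DrawToRend draws that material into the persistent target.
; moveRT moves the actor in XY to the player position, snapped to a texel grid (1/256 of capture width), then publishes its location to SnowMpc.
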(event `self.ReceiveTick`
  (params (DeltaSeconds :type "Float (single-precision)"))
  (`KismetMaterialLibrary.SetScalarParameterValue` "/Game/Snow/Snowtrail/SnowMpc.SnowMpc" "Size" (`SceneCaptureComponent2D.OrthoWidth` (`self.SceneCaptureComponent2D`)))
  (bind _returnvalue (`KismetMaterialLibrary.CreateDynamicMaterialInstance` "/Game/Snow/Snowtrail/Drawtopersistent.Drawtopersistent"))
  (set `self.DrawToPers` _returnvalue)
  (`KismetRenderingLibrary.ClearRenderTarget2D` "/Game/Snow/Snowtrail/RenderTarget.RenderTarget")
  (`KismetRenderingLibrary.ClearRenderTarget2D` "/Game/Snow/Snowtrail/RenderTargetpersis.RenderTargetpersis"))

(event `DrawToRend`
  (`KismetRenderingLibrary.DrawMaterialToRenderTarget` "/Game/Snow/Snowtrail/RenderTargetpersis.RenderTargetpersis" (`self.DrawToPers`)))

(event `moveRT`
  (bind (_returnvalue_x _returnvalue_y) (`KismetMathLibrary.BreakVector` (`self.K2_GetActorLocation` (`GameplayStatics.GetPlayerCharacter` 0))))
  (bind (_returnvalue_x_2 _returnvalue_y_2) (`KismetMathLibrary.BreakVector` (- (`self.SnapPixelToGrid` _returnvalue_x (* (`SceneCaptureComponent2D.OrthoWidth` (`self.SceneCaptureComponent2D`)) (/ 1.0 256.0)) _returnvalue_y) (`self.K2_GetActorLocation`))))
  (bind _output_get (set `self.Moveoffset` (`KismetMathLibrary.MakeVector2D` _returnvalue_x_2 _returnvalue_y_2)))
  (`self.K2_AddActorWorldOffset` (`KismetMathLibrary.MakeVector` (`KismetMathLibrary.BreakVector2D` _output_get) (`.Y` (`KismetMathLibrary.BreakVector2D` _output_get))))
  (`KismetMaterialLibrary.SetVectorParameterValue` "/Game/Snow/Snowtrail/SnowMpc.SnowMpc" "Capturelocation" (`KismetMathLibrary.Conv_VectorToLinearColor` (`self.K2_GetActorLocation`))))

(fn `UserConstructionScript`)