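; Snow render target actor that draws into a persistent render target, likely to record surface deformation.
; Its setup runs on Tick, not BeginPlay: it writes the scene capture's ortho width to SnowMPC, recreates the DrawToPersistent dynamic material and clears both render targets.
; Tick also re-sets a looping DrawToRT timer, which draws that material into the persistent target.
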(event `self.ReceiveTick`
  (params (DeltaSeconds :type "Float (single-precision)"))
  (`|ExecutionSequence`
    (:`then_0`
      (`KismetMaterialLibrary.SetScalarParameterValue` "/Game/Snow/SnowMPC.SnowMPC" "Size" (`SceneCaptureComponent2D.OrthoWidth` (`self.SceneCaptureComponent2D`)))
      (bind _returnvalue (`KismetMaterialLibrary.CreateDynamicMaterialInstance` "/Game/Snow/DrawToPersistent.DrawToPersistent"))
      (set `self.DrawToPMat` _returnvalue)
      (`KismetRenderingLibrary.ClearRenderTarget2D` "/Game/Snow/RenderTarget.RenderTarget")
      (`KismetRenderingLibrary.ClearRenderTarget2D` "/Game/Snow/RenderTargetPersistent.RenderTargetPersistent"))
    (:`then_1`
      (`KismetSystemLibrary.K2_SetTimer` null "DrawToRT" 0.01 true))))

(event `self.ReceiveBeginPlay`)

(event `DrawToRT`
  (`KismetRenderingLibrary.DrawMaterialToRenderTarget` "/Game/Snow/RenderTargetPersistent.RenderTargetPersistent" (`self.DrawToPMat`)))

(fn `UserConstructionScript`)